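; BP_BatteryCharacter_Code is the Blueprint layer of the BatteryCollector player character, tinting its body according to remaining power.
; The construction script creates a dynamic material instance on the mesh's first material slot and stores it.
; PowerChangeEffect lerps the BodyColor parameter from blue toward orange using the clamped ratio of current to initial power.
; BeginPlay, ActorBeginOverlap and Tick are empty.
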(event `self.PowerChangeEffect`
  (`MaterialInstanceDynamic.SetVectorParameterValue` (`self.MID_Character`) "BodyColor" (`KismetMathLibrary.LinearColorLerp` (struct :`R` 0.057805 :`G` 0.048172 :`B` 0.863157 :`A` 1.0) (struct :`R` 0.896269 :`G` 0.376262 :`B` 0.135633 :`A` 1.0) (`KismetMathLibrary.FClamp` (/ (`self.GetCurrentPower`) (`self.GetInitialPower`))))))

(fn `UserConstructionScript`
  (bind _returnvalue (`PrimitiveComponent.CreateDynamicMaterialInstance` (`self.Mesh`) 0 null "None"))
  (set `self.MID_Character` _returnvalue))