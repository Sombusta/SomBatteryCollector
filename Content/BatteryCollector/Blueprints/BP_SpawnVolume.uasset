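; BP_SpawnVolume is a battery spawner that drops BP_Battery actors at random points and rotations within the bounds of its WhereToSpawn component.
; SetSpawningActive starts or clears a looping timer that calls SpawnPickup, using a random delay between limits set in the Construction Script.
; SpawnPickup re-rolls and prints the delay, but the timer keeps its first interval because the rescheduling nodes are disconnected.
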(event `SetSpawningActive`
  (params (bShouldSpawn :type Boolean))
  (if bShouldSpawn
    (bind _output_get (set `self.SpawnDelay` (`KismetMathLibrary.RandomFloatInRange` (`self.SpawnDelayLow`) (`self.SpawnDelayHigh`))))
    (set `self.CountdownTime` (`KismetMathLibrary.FTrunc` _output_get))
    (bind _returnvalue (`KismetSystemLibrary.K2_SetTimerDelegate` (delegate `SpawnPickup`) (`self.SpawnDelay`) true))
    (set `self.SpawnerTimer` _returnvalue)
    (else
      (`KismetSystemLibrary.K2_ClearAndInvalidateTimerHandle` (`self.SpawnerTimer`)))))

(event `SpawnPickup`
  (`|SpawnActorFromClass` "/Game/BatteryCollector/Blueprints/BP_Battery.BP_Battery_C" (`KismetMathLibrary.MakeTransform` (`self.GetRandomPointInVolume`) (`KismetMathLibrary.MakeRotator` (`KismetMathLibrary.RandomFloatInRange` 0.0 360.0) (`KismetMathLibrary.RandomFloatInRange` 0.0 360.0) (`KismetMathLibrary.RandomFloatInRange` 0.0 360.0))) "Undefined" "OverrideRootScale" null null)
  (bind _output_get (set `self.SpawnDelay` (`KismetMathLibrary.RandomFloatInRange` (`self.SpawnDelayLow`) (`self.SpawnDelayHigh`))))
  (`KismetSystemLibrary.PrintString` (`KismetStringLibrary.Conv_DoubleToString` _output_get)))

(fn `GetRandomPointInVolume`
  (returns (RadomVector :type "Vector Structure"))
  (bind (_origin _boxextent) (`KismetSystemLibrary.GetComponentBounds` (`self.WhereToSpawn`)))
  (return (`KismetMathLibrary.RandomPointInBoundingBox` _origin _boxextent)))

(fn `UserConstructionScript`
  (set `self.SpawnDelayLow` 1.0)
  (set `self.SpawnDelayHigh` 4.5))