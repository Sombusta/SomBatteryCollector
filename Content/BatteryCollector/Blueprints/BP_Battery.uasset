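; BP_Battery is a collectible battery pickup whose construction script sets its BatteryPower.
; On collection it attaches an electricity beam emitter to PickupMesh, targeting the player character's spine socket.
; A short Delay loop keeps updating the beam target to follow the player, while a parallel one-second Delay postpones the parent WasCollected logic.
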(event `self.WasCollected`
  (bind _returnvalue (`GameplayStatics.SpawnEmitterAttached` "/Game/BatteryCollector/Assets/Effects/Particles/P_electricityc_BatteryCollector.P_electricityc_BatteryCollector" (`self.PickupMesh`) "None" (0.0 0.0 0.0) (struct) (1.0 1.0 1.0) "SnapToTargetIncludingScale"))
  (`ParticleSystemComponent.SetBeamTargetPoint` _returnvalue 0 (`SceneComponent.GetSocketLocation` (`Character.Mesh` (`GameplayStatics.GetPlayerCharacter` 0)) "spine_02") 0 :!label _label)
  (`|ExecutionSequence`
    (:`then_0`
      (`KismetSystemLibrary.Delay` 1.0)
      (`parent.WasCollected`))
    (:`then_1`
      (`KismetSystemLibrary.Delay` 0.01)
      (goto _label))))

(fn `UserConstructionScript`
  (`parent.UserConstructionScript`)
  (set `self.BatteryPower` 150.0))